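; BP_3dMap is a miniature 3D map that mirrors the player pawn with its Drone component.
; Each tick it sets the Drone's relative location to the pawn's world location scaled down by 1000.
; The Drone's relative rotation is rebuilt from the pawn's forward vector, so roll is dropped.
; Logic to mark DeliveryTarget actors on the map is unfinished and never runs.
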(event `self.ReceiveTick`
  (params (DeltaSeconds :type "Float (single-precision)"))
  (bind _returnvalue (`GameplayStatics.GetPlayerPawn` 0))
  (`|ExecutionSequence`
    (:`then_0`
      (`SceneComponent.K2_SetRelativeLocation` (`self.drone`) (/ (`self.K2_GetActorLocation` _returnvalue) (1000.0 1000.0 1000.0)) false false)
      (`SceneComponent.K2_SetRelativeRotation` (`self.drone`) (`KismetMathLibrary.Conv_VectorToRotator` (/ (`KismetMathLibrary.Conv_RotatorToVector` (`self.K2_GetActorRotation` _returnvalue)) (100.0 100.0 100.0))) false false))))

(fn `UserConstructionScript`)