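; BP_Billboard is an actor whose MaterialBillboard sprite is resized according to its distance from the first player's pawn.
; Every Tick sets the first element's width and height proportional to that distance, with a smaller factor beyond a near threshold, so size drops abruptly there.
; The edited element is written back through SetElements as the only entry in the array.
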(event `self.ReceiveTick`
  (params (DeltaSeconds :type "Float (single-precision)"))
  (bind _returnvalue (`self.GetDistanceTo` (`GameplayStatics.GetPlayerPawn` 0)))
  (bind _returnvalue_2 (/ _returnvalue 30.0))
  (bind _returnvalue_3 (/ _returnvalue 10.0))
  (bind _output (`|GetArrayItem` (`MaterialBillboardComponent.Elements` (`self.MaterialBillboard`))))
  (if (< _returnvalue 1000.0)
    (bind _structout (setmembers `MaterialSpriteElement` :`StructRef` _output :`BaseSizeX` _returnvalue_3 :`BaseSizeY` _returnvalue_3))
    (`MaterialBillboardComponent.SetElements` (`self.MaterialBillboard`) (`|MakeArray` _structout))
    (else
      (bind _structout_2 (setmembers `MaterialSpriteElement` :`StructRef` _output :`BaseSizeX` _returnvalue_2 :`BaseSizeY` _returnvalue_2))
      (`MaterialBillboardComponent.SetElements` (`self.MaterialBillboard`) (`|MakeArray` _structout_2)))))

(fn `UserConstructionScript`)