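; Pathfinder actor that builds an arched trail of rings linked by cables toward an Xmark target at BeginPlay.
; It moves the spline's end point to the target and lifts the middle point at half the spline's length to form the arc.
; It spawns five rings evenly along the first half of the spline, adding a cable component at each.
; Each cable's end is set to the preceding ring, with the first indexing before the list start.
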(event `self.ReceiveBeginPlay`
  (bind _spline (`self.Spline`))
  (bind (_returnvalue_x _returnvalue_y _returnvalue_z) (`KismetMathLibrary.BreakVector` (`SplineComponent.GetLocationAtSplinePoint` (`self.Spline`) 0 "Local")))
  (bind (_returnvalue_x_2 _returnvalue_y_2) (`KismetMathLibrary.BreakVector` (`SplineComponent.GetLocationAtDistanceAlongSpline` (`self.Spline`) (/ (`SplineComponent.GetDistanceAlongSplineAtSplinePoint` (`self.Spline`) 2) 2.0) "Local")))
  ;[0 0 0] calculate spline mid distance to target
  (`SplineComponent.SetLocationAtSplinePoint` (`self.Spline`) 2 (`self.K2_GetActorLocation` (`self.xmark`)) "World" true)
  (`SplineComponent.SetLocationAtSplinePoint` (`self.Spline`) 1 (`KismetMathLibrary.MakeVector` _returnvalue_x_2 _returnvalue_y_2 (+ _returnvalue_z 500.0)) "Local" true)
  ;[0.2257 1 0.8599] sets rings at distances along spline
  (for _index (range 1 6)
    (bind _returnvalue (`|SpawnActorFromClass` "/Game/Myblueprints/Ring_actor.Ring_actor_C" (`KismetMathLibrary.MakeTransform` (`SplineComponent.GetLocationAtDistanceAlongSpline` _spline (* (`SplineComponent.GetDistanceAlongSplineAtSplinePoint` _spline 2) (* (`KismetMathLibrary.Conv_IntToDouble` _index) 0.1)) "World")) "Undefined" "OverrideRootScale" null null))
    ;[0 0.3919 1] spawn cable actors
    (`KismetArrayLibrary.Array_Add` (`self.ring List`) _returnvalue)
    (bind _returnvalue_2 (`AddComponent|NODE_AddCableComponent-0`))
    (`KismetArrayLibrary.Array_Add` (`self.Cable list`) _returnvalue_2)
    (`SceneComponent.K2_SetWorldLocation` _returnvalue_2 (`self.K2_GetActorLocation` _returnvalue) false false))
  ;[0 0 0] attatch cables together
  (for _index_2 (range 5)
    (`CableComponent.SetAttachEndTo` (`|GetArrayItem` (`self.Cable list`) _index_2) (`|GetArrayItem` (`self.ring List`) (- _index_2 1)) "None" "None")))

(fn `UserConstructionScript`)